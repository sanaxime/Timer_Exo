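; BP_Vitrine is a procedural display-case actor that fills a showcase mesh with randomly scattered props, built entirely in the Construction Script.
; HISM01 holds the single case instance, whose local bounds set the area where HISM02 spawns PropsCount prop instances at a shared height offset with random yaw.
; Each prop writes random RGB values into per-instance custom data, presumably for colour variation in the assigned material.
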(fn `UserConstructionScript`
  (bind _returnvalue (`KismetMathLibrary.RandomFloat`))
  (bind (_returnvalue_r _returnvalue_g _returnvalue_b) (break `LinearColor` (`KismetMathLibrary.MakeColor` _returnvalue _returnvalue _returnvalue)))
  (bind (_min _max) (`StaticMeshComponent.GetLocalBounds` (`self.HISM_01`)))
  (bind (_returnvalue_x _returnvalue_y) (`KismetMathLibrary.BreakVector` (- _max _min)))
  (`PrimitiveComponent.SetMaterial` (`self.HISM_02`) 0 (`self.Material`))
  (`StaticMeshComponent.SetStaticMesh` (`self.HISM_01`) (`self.Vitrine`))
  (`StaticMeshComponent.SetStaticMesh` (`self.HISM_02`) (`self.props1`))
  (set `self.Vitrine_x` _returnvalue_x)
  (set `self.Vitrine_y` _returnvalue_y)
  (`InstancedStaticMeshComponent.AddInstance` (`self.HISM_01`) (`KismetMathLibrary.MakeTransform` (0.0 0.0 0.0)) false)
  (for _ (range (`self.props_count`))
    (bind _returnvalue_2 (`InstancedStaticMeshComponent.AddInstance` (`self.HISM_02`) (`KismetMathLibrary.MakeTransform` (`KismetMathLibrary.MakeVector` (`KismetMathLibrary.RandomFloatInRange` (- (/ (`self.Vitrine_x`) 3.0) (* (/ (`self.Vitrine_x`) 3.0) 2.0)) (/ (`self.Vitrine_x`) 3.0)) (`KismetMathLibrary.RandomFloatInRange` (- (/ (`self.Vitrine_y`) 3.0) (* (/ (`self.Vitrine_y`) 4.0) 2.0)) (/ (`self.Vitrine_y`) 3.0)) (+ 0.0 (`self.decale_z`))) (`KismetMathLibrary.MakeRotator` 0.0 0.0 (`KismetMathLibrary.RandomFloatInRange` 0.0 360.0))) false))
    (`InstancedStaticMeshComponent.SetCustomDataValue` (`self.HISM_02`) _returnvalue_2 0 _returnvalue_r false)
    (`InstancedStaticMeshComponent.SetCustomDataValue` (`self.HISM_02`) _returnvalue_2 1 _returnvalue_g false)
    (`InstancedStaticMeshComponent.SetCustomDataValue` (`self.HISM_02`) _returnvalue_2 2 _returnvalue_b false)))