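; Actor that procedurally builds a vertical tower of stacked, progressively rotated mesh instances with random colors.
; The Construction Script assigns the mesh and material to a HISM component, then stacks instances by the mesh's bounds height.
; Yaw increments spread about one full turn across the tower's length.
; Each instance receives random RGB through three per-instance custom data floats, while the event graph holds no active logic.
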(fn `UserConstructionScript`
  (bind _returnvalue (`KismetMathLibrary.RandomFloat`))
  (bind (_min _max) (`StaticMeshComponent.GetLocalBounds` (`self.HISM_00`)))
  (bind (_returnvalue_r _returnvalue_g _returnvalue_b) (break `LinearColor` (`KismetMathLibrary.MakeColor` _returnvalue _returnvalue _returnvalue)))
  (bind (_returnvalue_x _returnvalue_y _returnvalue_z) (`KismetMathLibrary.BreakVector` (- _max _min)))
  (`PrimitiveComponent.SetMaterial` (`self.HISM_00`) 0 (`self.Material`))
  (`StaticMeshComponent.SetStaticMesh` (`self.HISM_00`) (`self.static_mesh`))
  (set `self.cube_z` _returnvalue_z)
  (set `self.Decal_z` (/ (`self.cube_z`) 2.0))
  (set `self.Rotation_value` (`KismetMathLibrary.Conv_IntToDouble` (/ 360 (- (`self.Tower_Lenght_z`) 1))))
  (if (> (`self.Tower_Lenght_z`) 0)
    (for _index (range (`self.Tower_Lenght_z`))
      (bind _output_get (set `self.cube_lenght_z` (+ (* _index (`KismetMathLibrary.MakeVector` 0.0 0.0 (`self.cube_z`))) (`KismetMathLibrary.MakeVector` 0.0 0.0 (`self.Decal_z`)))))
      (bind _returnvalue_2 (`InstancedStaticMeshComponent.AddInstance` (`self.HISM_00`) (`KismetMathLibrary.MakeTransform` _output_get (`KismetMathLibrary.MakeRotator` 0.0 0.0 (`self.rotation_cube`))) false))
      (set `self.rotation_cube` (+ (`self.Rotation_value`) (`self.rotation_cube`)))
      (`InstancedStaticMeshComponent.SetCustomDataValue` (`self.HISM_00`) _returnvalue_2 0 _returnvalue_r false)
      (`InstancedStaticMeshComponent.SetCustomDataValue` (`self.HISM_00`) _returnvalue_2 1 _returnvalue_g false)
      (`InstancedStaticMeshComponent.SetCustomDataValue` (`self.HISM_00`) _returnvalue_2 2 _returnvalue_b false))))