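; BP_Cube_Shape builds a hollow box out of instanced copies of a static mesh.
; The Construction Script clears the HISM, reads the mesh bounds for spacing, then loops over Z, X and Y counts, adding local-space instances only on outer layers, raised by OffsetZ.
; The far Y face is tested against WallSizeX rather than WallSizeY, so the shell is correct only when both match.
; The event graph has no active logic.
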(fn `UserConstructionScript`
  (bind _index_x (`self.Index X`))
  (bind _index_y (`self.Index Y`))
  (bind (_min _max) (`StaticMeshComponent.GetLocalBounds` (`self.HISM`)))
  (bind (_returnvalue_x _returnvalue_y _returnvalue_z) (`KismetMathLibrary.BreakVector` (- _max _min)))
  (`InstancedStaticMeshComponent.ClearInstances` (`self.HISM`))
  (`StaticMeshComponent.SetStaticMesh` (`self.HISM`) (`self.Static Mesh`))
  (if (and (> (`self.wall_size_z`) 0) (> (`self.wall_size_x`) 0) (> (`self.wall_size_y`) 0))
    (set `self.x_cube_size` _returnvalue_x)
    (set `self.y_cube_size` _returnvalue_y)
    (set `self.z_cube_size` _returnvalue_z)
    (for _index (range (`self.wall_size_z`))
      (bind _output_get (set `self.Index Z` _index))
      (set `self.Location z` (`KismetMathLibrary.MakeVector` 0.0 0.0 (+ (* _output_get (`self.z_cube_size`)) (`self.Offset Z`))))
      (for _index_2 (range (`self.wall_size_x`))
        (bind _output_get_2 (set `self.Index X` _index_2))
        (set `self.Location x` (`KismetMathLibrary.MakeVector` (* _output_get_2 (`self.x_cube_size`))))
        (for _index_3 (range (`self.wall_size_y`))
          (bind _output_get_3 (set `self.Index Y` _index_3))
          (set `self.Location y` (`KismetMathLibrary.MakeVector` 0.0 (* _output_get_3 (`self.y_cube_size`))))
          (if (or (or (== (`self.Index Z`) 0) (== (`self.Index Z`) (- (`self.wall_size_z`) 1))) (or (== _index_x 0) (== _index_x (- (`self.wall_size_x`) 1))) (or (== _index_y 0) (== _index_y (- (`self.wall_size_x`) 1))))
            (`InstancedStaticMeshComponent.AddInstance` (`self.HISM`) (`KismetMathLibrary.MakeTransform` (+ (`self.Location z`) (`self.Location y`) (`self.Location x`))) false)))))))