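; BP_Wall is a construction-script actor that builds a box outline of instanced cubes, sized by WallSizeX, WallSizeY and WallSizeZ.
; It clears HISM00, takes cube spacing from the mesh's local bounds, then loops X, Z and Y, adding instances along edges only.
; CountX and CountZ detect the ends; CountZ is never reset, so the far X end gets vertical columns without Y rows.
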(fn `UserConstructionScript`
  (bind (_min _max) (`StaticMeshComponent.GetLocalBounds` (`self.HISM 00`)))
  (bind (_returnvalue_x _returnvalue_y _returnvalue_z) (`KismetMathLibrary.BreakVector` (- _max _min)))
  (`InstancedStaticMeshComponent.ClearInstances` (`self.HISM 00`))
  (if (and (> (`self.wall_size_z`) 0) (> (`self.wall_size_x`) 0) (> (`self.wall_size_y`) 0))
    (set `self.x_cube_size` _returnvalue_x)
    (set `self.y_cube_size` _returnvalue_y)
    (set `self.z_cube_size` _returnvalue_z)
    (for _index (range (`self.wall_size_x`))
      (set `self.cube_x` (* _index (`KismetMathLibrary.MakeVector` (`self.x_cube_size`))))
      (if (or (== (`self.count_x`) 0.0) (== (`self.count_x`) (- (`self.wall_size_x`) 1)))
        (set `self.count_x` (+ (`self.count_x`) 1.0))
        (for _index_2 (range (`self.wall_size_z`))
          (set `self.cube_z` (* _index_2 (`KismetMathLibrary.MakeVector` 0.0 0.0 (`self.z_cube_size`))))
          (if (or (== (`self.count_z`) 0.0) (== (`self.count_z`) (- (`self.wall_size_z`) 1)))
            (set `self.count_z` (+ (`self.count_z`) 1.0))
            (for _index_3 (range (`self.wall_size_y`))
              (set `self.cube_y` (* _index_3 (`KismetMathLibrary.MakeVector` 0.0 (`self.y_cube_size`))))
              (`InstancedStaticMeshComponent.AddInstance` (`self.HISM 00`) (`KismetMathLibrary.MakeTransform` (+ (`self.cube_x`) (`self.cube_z`) (`self.cube_y`))) false))
            (else
              (set `self.count_z` (+ (`self.count_z`) 1.0))
              (`InstancedStaticMeshComponent.AddInstance` (`self.HISM 00`) (`KismetMathLibrary.MakeTransform` (+ (`self.cube_x`) (`self.cube_z`))) false)
              (`InstancedStaticMeshComponent.AddInstance` (`self.HISM 00`) (`KismetMathLibrary.MakeTransform` (+ (`self.cube_x`) (`self.cube_z`) (`self.cube_y`))) false))))
        (else
          (set `self.count_x` (+ (`self.count_x`) 1.0))
          (`InstancedStaticMeshComponent.AddInstance` (`self.HISM 00`) (`KismetMathLibrary.MakeTransform` (`self.cube_x`)) false)
          (`InstancedStaticMeshComponent.AddInstance` (`self.HISM 00`) (`KismetMathLibrary.MakeTransform` (+ (`self.cube_x`) (`self.cube_z`))) false)
          (`InstancedStaticMeshComponent.AddInstance` (`self.HISM 00`) (`KismetMathLibrary.MakeTransform` (+ (`self.cube_x`) (`self.cube_y`))) false)
          (`InstancedStaticMeshComponent.AddInstance` (`self.HISM 00`) (`KismetMathLibrary.MakeTransform` (+ (`self.cube_x`) (`self.cube_y`) (`self.cube_z`))) false))))))