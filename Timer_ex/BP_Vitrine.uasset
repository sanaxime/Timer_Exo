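; BP_Vitrine is a procedural display case that fills itself with randomly scattered props in its construction script.
; One HISM places the case mesh, while a second spawns PropsCount props at random XY positions and yaws within a Box's extents, offset vertically by DecaleZ.
; Each prop gets random RGB values as per-instance custom data, presumably for color variation in the assigned material.
; The event graph has no active logic.
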(fn `UserConstructionScript`
  (bind _returnvalue (`KismetMathLibrary.RandomFloat`))
  (bind _box (`self.Box`))
  (bind (_returnvalue_x _returnvalue_y _returnvalue_z) (`KismetMathLibrary.BreakVector` (`SceneComponent.K2_GetComponentLocation` _box)))
  (bind (_returnvalue_r _returnvalue_g _returnvalue_b) (break `LinearColor` (`KismetMathLibrary.MakeColor` _returnvalue _returnvalue _returnvalue)))
  (bind (_min _max) (`StaticMeshComponent.GetLocalBounds` (`self.HISM_01`)))
  (bind (_boxextent_x _boxextent_y) (`KismetMathLibrary.BreakVector` (`BoxComponent.BoxExtent` _box)))
  (bind (_returnvalue_x_2 _returnvalue_y_2) (`KismetMathLibrary.BreakVector` (- _max _min)))
  (`PrimitiveComponent.SetMaterial` (`self.HISM_02`) 0 (`self.Material`))
  (`StaticMeshComponent.SetStaticMesh` (`self.HISM_01`) (`self.Vitrine`))
  (`StaticMeshComponent.SetStaticMesh` (`self.HISM_02`) (`self.props1`))
  (set `self.Vitrine_x` _returnvalue_x_2)
  (set `self.Vitrine_y` _returnvalue_y_2)
  (`InstancedStaticMeshComponent.AddInstance` (`self.HISM_01`) (`KismetMathLibrary.MakeTransform` (0.0 0.0 0.0)) false)
  (`SceneComponent.K2_SetWorldLocation` (`self.Box`) (0.0 0.0 0.0) false false)
  (for _ (range (`self.props_count`))
    (bind _returnvalue_2 (`InstancedStaticMeshComponent.AddInstance` (`self.HISM_02`) (`KismetMathLibrary.MakeTransform` (`KismetMathLibrary.MakeVector` (`KismetMathLibrary.RandomFloatInRange` (- _returnvalue_x _boxextent_x) (+ _returnvalue_x _boxextent_x)) (`KismetMathLibrary.RandomFloatInRange` (- _returnvalue_y _boxextent_y) (+ _returnvalue_y _boxextent_y)) (+ _returnvalue_z (`self.decale_z`))) (`KismetMathLibrary.MakeRotator` 0.0 0.0 (`KismetMathLibrary.RandomFloatInRange` 0.0 360.0))) false))
    (`InstancedStaticMeshComponent.SetCustomDataValue` (`self.HISM_02`) _returnvalue_2 0 _returnvalue_r false)
    (`InstancedStaticMeshComponent.SetCustomDataValue` (`self.HISM_02`) _returnvalue_2 1 _returnvalue_g false)
    (`InstancedStaticMeshComponent.SetCustomDataValue` (`self.HISM_02`) _returnvalue_2 2 _returnvalue_b false)))